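; BP_Dynamic_Enemy is a hazard enemy that patrols back and forth along the Y axis and hurts the player on contact.
; Each tick moves the Enemy component by a local Y offset without sweep, picking a random speed toward the other side whenever its world Y passes either fixed bound.
; A component hit against BP_ThirdPersonCharacter applies damage to that character.
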(event OnComponentHit(Enemy)
  (params (HitComponent :type Primitive%20Component%20Object%20Reference) (OtherActor :type Actor%20Object%20Reference) (OtherComp :type Primitive%20Component%20Object%20Reference) (NormalImpulse :type Vector :default "0, 0, 0") (Hit :type Hit%20Result%20Structure%20%28by%20ref%29))
  ;[1 1 1] Apply damage when hit player
  (bind _asbp_third_person_character (Utilities|Casting|CastToBP_ThirdPersonCharacter OtherActor))
  (Game|Damage|ApplyDamage _asbp_third_person_character 5e+01 0 0))

(event EventBeginPlay
  ;[1 1 1] Set initial offset
  (Variables|Default|SetOffset (Math|Random|RandomFloatinRange -7e+02 -5e+02)))

(event EventTick
  (params (DeltaSeconds :type Float%20%28single-precision%29))
  (bind _enemy (Variables|Default|GetEnemy))
  (bind _returnvalue (Transformation|GetWorldTransform _enemy))
  (bind _location (Math|Transform|BreakTransform _returnvalue))
  (bind _y (Math|Vector|BreakVector _location))
  ;[1 1 1] Add local offset every tick
  (if (< _y 1.1e+03)
    (Variables|Default|SetOffset (Math|Random|RandomFloatinRange 5e+02 7e+02))
    (elif (> _y 2.6e+03)
      (Variables|Default|SetOffset (Math|Random|RandomFloatinRange -7e+02 -5e+02))))
  (Transformation|AddLocalOffset _enemy (Math|Vector|MakeVector 0.0 (* (Variables|Default|GetOffset) DeltaSeconds) 0.0) false false))

(fn ConstructionScript)