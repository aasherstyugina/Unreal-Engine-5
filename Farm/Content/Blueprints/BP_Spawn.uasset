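; Level spawner that builds a run of randomly counted BP_Room segments, starting with an easy room at BeginPlay.
; Each room gets a reference back to this spawner; SpawnRoom chains the next one from the last room's SpawnCoords.
; Rooms are filled at random positions with tree-trunk enemies, plus stone enemies and meat heals in hard rooms.
; The final room also receives the victory stone.
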(event EventBeginPlay
  ;[1 1 1] Spawn first easy room
  (Variables|Default|SetCountRooms (Math|Random|RandomIntegerinRange 6 10))
  (CallFunction|SpawnNextRoom "1000.000000,2700.000000,260.000000" true))

(fn ConstructionScript)

(fn SpawnNextRoom
  (params (Location :type Vector) (IsEasy :type Boolean))
  ;[1 1 1] Spawn next room
  ;;[1 1 1] Draw count of left rooms
  (Development|PrintString (Utilities|String|BuildString(Integer) "Rooms left:" "" (Variables|Default|GetCountRooms)) true true "(R=0.275000,G=0.000000,B=0.001786,A=1.000000)")
  ;;[1 1 1] Spawn new room
  (if (> (Variables|Default|GetCountRooms) 0)
    (bind _returnvalue (Game|SpawnActorfromClass "/Game/Blueprints/BP_Room.BP_Room_C" (Math|Transform|MakeTransform (+ Location "0,15.000000,0")) "Undefined" 0 0))
    (bind _output_get (Variables|Default|SetLastRoom _returnvalue))
    (Variables|/Game/Blueprints/BP_Room.BP_Room_C|SetSpawner _output_get self)
    (Variables|/Game/Blueprints/BP_Room.BP_Room_C|SetIsEasy _output_get IsEasy)
    ;;[1 1 1] Check if it is last room
    (if (== (Variables|Default|GetCountRooms) 1)
      (CallFunction|SpawnVictoryStone))
    (if (Variables|/Game/Blueprints/BP_Room.BP_Room_C|GetIsEasy (Variables|Default|GetLastRoom))
      ;;[1 1 1] Create easy traps
      (for _index (range 0 (Math|Random|RandomIntegerinRange 3 5))
        (CallFunction|SpawnTreeTrunk))
      (else
        ;;[1 1 1] Create hard traps
        (for _index_2 (range 0 (Math|Random|RandomIntegerinRange 3 5))
          (CallFunction|SpawnTreeTrunk))
        (for _index_3 (range 0 (Math|Random|RandomIntegerinRange 15 25))
          (CallFunction|SpawnStones false))
        (for _index_4 (range 0 (Math|Random|RandomIntegerinRange 4 7))
          (CallFunction|SpawnMeat))))
    (Variables|Default|SetCountRooms (- (Variables|Default|GetCountRooms) 1))))

(fn SpawnRoom
  (params (IsEasy :type Boolean))
  ;[1 1 1] Send location to spawn next room
  (CallFunction|SpawnNextRoom (+ (Transformation|GetWorldLocation (Variables|/Game/Blueprints/BP_Room.BP_Room_C|GetSpawnCoords (Variables|Default|GetLastRoom))) (Math|Vector|MakeVector -1.5e+03 8e+02 0.0)) IsEasy))

(fn SpawnTreeTrunk
  (bind _lastroom (Variables|Default|GetLastRoom))
  (bind _rootcomponent (Variables|/Script/Engine.Actor|GetRootComponent _lastroom))
  (bind _returnvalue (Transformation|GetWorldLocation _rootcomponent))
  (bind (_x _y _z) (Math|Vector|BreakVector _returnvalue))
  ;[1 1 1] Spawn treetrunk
  (Game|SpawnActorfromClass "/Game/Blueprints/BP_Dynamic_Enemy.BP_Dynamic_Enemy_C" (Math|Conversions|ToTransform(Vector) (Math|Vector|MakeVector (+ _x (Math|Random|RandomFloatinRange -2.7e+03 -1.5e+03)) (Math|Random|RandomFloatinRange 1.1e+03 2.5e+03) _z)) "Undefined" 0 0))

(fn SpawnStones
  (params (NewParam :type Boolean))
  (bind _lastroom (Variables|Default|GetLastRoom))
  (bind _rootcomponent (Variables|/Script/Engine.Actor|GetRootComponent _lastroom))
  (bind _returnvalue (Transformation|GetWorldLocation _rootcomponent))
  (bind (_x _y _z) (Math|Vector|BreakVector _returnvalue))
  ;[1 1 1] Spawn stone
  (Game|SpawnActorfromClass "/Game/Blueprints/BP_Static_Enemy.BP_Static_Enemy_C" (Math|Conversions|ToTransform(Vector) (Math|Vector|MakeVector (+ _x (Math|Random|RandomFloatinRange -2.7e+03 -1.5e+03)) (Math|Random|RandomFloatinRange 1e+03 2.6e+03) _z)) "Undefined" 0 0))

(fn SpawnVictoryStone
  ;[1 1 1] Spawn victory stone
  ;;[1 1 1] Set location
  (Game|SpawnActorfromClass "/Game/Blueprints/BP_Victory_Stone.BP_Victory_Stone_C" (Math|Conversions|ToTransform(Vector) (+ (Transformation|GetWorldLocation (Variables|/Script/Engine.Actor|GetRootComponent (Variables|Default|GetLastRoom))) (Math|Vector|MakeVector -2.5e+03 -1e+03 1e+02))) "Undefined" 0 0))

(fn SpawnMeat
  (bind _lastroom (Variables|Default|GetLastRoom))
  (bind _rootcomponent (Variables|/Script/Engine.Actor|GetRootComponent _lastroom))
  (bind _returnvalue (Transformation|GetWorldLocation _rootcomponent))
  (bind (_x _y _z) (Math|Vector|BreakVector _returnvalue))
  ;[1 1 1] Spawn meat
  (Game|SpawnActorfromClass "/Game/Blueprints/BP_Heal.BP_Heal_C" (Math|Conversions|ToTransform(Vector) (Math|Vector|MakeVector (+ _x (Math|Random|RandomFloatinRange -2.7e+03 -1.5e+03)) (Math|Random|RandomFloatinRange 1e+03 2.6e+03) _z)) "Undefined" 0 0))